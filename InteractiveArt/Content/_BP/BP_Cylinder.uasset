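; BP_Cylinder is a physics cylinder that recursively shatters into smaller copies of itself.
; After a delay, shorter for the first piece, it bursts in Niagara, spawns children at eight scene-component points with scale relative to its own, then destroys itself.
; Each instance rolls its own random generation limit, so branches stop at varying depths.
; Generation shifts the dynamic material's hue, and spawned pieces get a random impulse and brief emissive flash.
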(event `self.ReceiveBeginPlay`
  (bind _spawnlocations (`self.SpawnLocations`))
  (bind _mid_cube (`self.MID_Cube`))
  (`KismetArrayLibrary.Array_Add` _spawnlocations (`self.P1`))
  (`KismetArrayLibrary.Array_Add` _spawnlocations (`self.P2`))
  (`KismetArrayLibrary.Array_Add` _spawnlocations (`self.P3`))
  (`KismetArrayLibrary.Array_Add` _spawnlocations (`self.P4`))
  (`KismetArrayLibrary.Array_Add` _spawnlocations (`self.P5`))
  (`KismetArrayLibrary.Array_Add` _spawnlocations (`self.P6`))
  (`KismetArrayLibrary.Array_Add` _spawnlocations (`self.P7`))
  (`KismetArrayLibrary.Array_Add` _spawnlocations (`self.P8`))
  (bind _returnvalue (`PrimitiveComponent.CreateDynamicMaterialInstance` (`self.Cylinder`) 0 "/Game/_MAt/MI_Cylinder.MI_Cylinder" "None"))
  (bind _output_get (set `self.MID_Cube` _returnvalue))
  (`MaterialInstanceDynamic.SetScalarParameterValue` _output_get "HueOffset" (`KismetMathLibrary.Conv_IntToDouble` (`self.Generation`)))
  (set `self.MaxGenerations` (`KismetMathLibrary.RandomIntegerInRange` 1 4))
  (if (`self.FirstCube?`)
    (`self.StartSplit`)
    (else
      (`PrimitiveComponent.AddImpulse` (`self.Cylinder`) (* (`KismetMathLibrary.RandomUnitVector`) (`self.ImpulseScalar`)) "None" true)
      (`self.StartSplit`)
      ;[1 1 1] Emission Flashing Effect
      (`MaterialInstanceDynamic.SetScalarParameterValue` _mid_cube "Emission" 5.0)
      (`KismetSystemLibrary.Delay` 0.1)
      (`MaterialInstanceDynamic.SetScalarParameterValue` _mid_cube "Emission" 0.0))))

(event `StartSplit`
  (bind _result (`/Engine/EditorBlueprintResources/StandardMacros.IncrementInt` (`self.Generation`))
    (:`  `
      (if (<= _result (`self.MaxGenerations`))
        (if (`self.FirstCube?`)
          (`KismetSystemLibrary.Delay` 0.2)
          (else
            (`KismetSystemLibrary.Delay` (`KismetMathLibrary.RandomFloatInRange` 1.0 4.0))))
        (`self.DisableParentCube`)
        (`self.SpawnCubes`)))))

(event `SpawnCubes`
  (bind (_returnvalue_location _returnvalue_rotation _returnvalue_scale) (`KismetMathLibrary.BreakTransform` (`self.GetTransform`)))
  (`NiagaraFunctionLibrary.SpawnSystemAtLocation` "/Game/_FX/NS_Burst.NS_Burst" _returnvalue_location _returnvalue_rotation _returnvalue_scale)
  (for _array_element (`self.SpawnLocations`)
    (`|SpawnActorFromClass` "BP_Cylinder_C" (`KismetMathLibrary.MakeTransform` (`SceneComponent.K2_GetComponentLocation` _array_element) (`SceneComponent.K2_GetComponentRotation` _array_element) (* (`SceneComponent.RelativeScale3D` _array_element) (`self.GetActorScale3D`))) "AlwaysSpawn" "MultiplyWithRoot" null (`self.Generation`) null))
  (`self.K2_DestroyActor`))

(fn `DisableParentCube`
  (bind _cylinder (`self.Cylinder`))
  (`PrimitiveComponent.SetSimulatePhysics` _cylinder false)
  (`PrimitiveComponent.SetCollisionEnabled` _cylinder "NoCollision")
  (`PrimitiveComponent.SetCollisionObjectType` _cylinder "ECC_WorldStatic"))

(fn `UserConstructionScript`)